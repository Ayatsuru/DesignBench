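; Debug test actor in the DesignBench tools that exercises queries on the EntityCatalogSubsystem.
; On BeginPlay it prints the display names of entities matching an Entity.Type.Prop gameplay tag query, then those from a hard-coded name search in red on screen.
; Unconnected match-all, match-any and match-none tag query nodes remain in the graph, and the construction script is empty.
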(event `self.ReceiveBeginPlay`
  (bind _returnvalue (subsystem `EntityCatalogSubsystem`))
  (for _array_element (`EntityCatalogSubsystem.GetEntitiesMatchingQuery` _returnvalue (make `GameplayTagQuery` (`BlueprintGameplayTagLibrary.MakeGameplayTagQuery` (struct :`TagDictionary` (struct :`(TagName` "Entity.Type.Prop") :`(TagName` "Entity.Capability.Explosive")) :`QueryTokenStream` "(0,1,5,2,2,1,0,3,1,1)" :`AutoDescription` " ALL(  ALL( Entity.Type.Prop ),  NONE( Entity.Capability.Explosive ) )"))))
    (`KismetSystemLibrary.PrintString` (`KismetTextLibrary.Conv_TextToString` (`EntityDefinition.DisplayName` _array_element))))
  (for _array_element_2 (`EntityCatalogSubsystem.SearchEntitiesByName` _returnvalue "atr")
    (`KismetSystemLibrary.PrintString` (`KismetTextLibrary.Conv_TextToString` (`EntityDefinition.DisplayName` _array_element_2)) true false (struct :`R` 1.0 :`B` 0.04085 :`A` 1.0) 10.0)))

(fn `UserConstructionScript`)